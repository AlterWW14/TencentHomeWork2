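; Ball actor that flies along its Direction at Speed and awards a point to the player who damages it.
; Tick moves it without sweep and drives a one-second Delay countdown shown on two text renders; expiry triggers nothing.
; On damage, the server waits a second, increments the instigator's MyPlayerState score, activates a particle and destroys the ball.
; Random countdown setup, radial force and a separate destroy are disconnected.
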(event EventTick
  (params (DeltaSeconds :type Float%20%28single-precision%29))
  (bind _returnvalue (Transformation|GetActorTransform))
  (bind (_location _rotation _scale) (Math|Transform|BreakTransform _returnvalue))
  (Transformation|SetActorTransform (Math|Transform|MakeTransform (+ (* (Math|Vector|Normalize (Variables|Default|GetDirection)) (* DeltaSeconds (Variables|Default|GetSpeed))) _location) _rotation _scale))
  (Utilities|FlowControl|Delay 1.0 :!label _label)
  (bind _output_get (Variables|Default|SetCountDown (- (Variables|Default|GetCountDown) 1)))
  (if (> _output_get -1)
    (Rendering|Components|TextRender|SetText (Variables|Default|GetTextRender) (Utilities|Text|ToText(Integer) _output_get))
    (goto _label)))

(event Game|Damage|EventAnyDamage
  (params (Damage :type Float%20%28single-precision%29) (DamageType :type Damage%20Type%20Object%20Reference) (InstigatedBy :type Controller%20Object%20Reference) (DamageCauser :type Actor%20Object%20Reference))
  (Development|PrintString "Hello")
  (Networking|SwitchHasAuthority
    (:Authority
      (Utilities|FlowControl|Delay 1.0)
      (bind _asmy_player_state (Utilities|Casting|CastToMyPlayerState (Variables|/Script/Engine.Controller|GetPlayerState InstigatedBy)))
      (Default|IncrementScore _asmy_player_state)
      (Components|Activation|SetActive (Variables|Default|GetParticleSystem) true false)
      (Actor|DestroyActor))))

(fn ConstructionScript)